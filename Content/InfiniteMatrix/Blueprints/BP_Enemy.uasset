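; BP_Enemy is an enemy actor that is destroyed when a projectile or the player overlaps its TriggerZo component.
; BeginPlay caches the first BP_Player found with GetAllActorsOfClass.
; A BP_Projectile hit updates that player's score and calls UpdateSpeed on the projectile before destroying the enemy.
; Player contact calls UpdateHealth on the player and destroys the enemy, while other actors are ignored.
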(event OnComponentBeginOverlap(TriggerZo)
  (params (OverlappedComponent :type Primitive%20Component%20Object%20Reference) (OtherActor :type Actor%20Object%20Reference) (OtherComp :type Primitive%20Component%20Object%20Reference) (OtherBodyIndex :type Integer) (bFromSweep :type Boolean) (SweepResult :type Hit%20Result%20Structure%20%28by%20ref%29))
  (if (== (Utilities|GetClass OtherActor) "/Game/InfiniteMatrix/Blueprints/BP_Projectile.BP_Projectile_C")
    (Default|UpdateScore (Variables|Default|Getplayer))
    (bind _asbp_projectile (Utilities|Casting|CastToBP_Projectile OtherActor))
    (Default|UpdateSpeed _asbp_projectile)
    (Actor|DestroyActor)
    (else
      (bind _asbp_player (Utilities|Casting|CastToBP_Player OtherActor))
      (Default|UpdateHealth _asbp_player)
      (Actor|DestroyActor))))

(event OnComponentEndOverlap(TriggerZo)
  (params (OverlappedComponent :type Primitive%20Component%20Object%20Reference) (OtherActor :type Actor%20Object%20Reference) (OtherComp :type Primitive%20Component%20Object%20Reference) (OtherBodyIndex :type Integer)))

(event EventBeginPlay
  (bind _outactors (Actor|GetAllActorsOfClass "/Game/InfiniteMatrix/Blueprints/BP_Player.BP_Player_C"))
  (Variables|Default|Setplayer (Utilities|Array|Get(acopy) _outactors)))

(event Collision|EventActorBeginOverlap
  (params (OtherActor :type Actor%20Object%20Reference)))

(event EventTick
  (params (DeltaSeconds :type Float%20%28single-precision%29)))

(fn ConstructionScript)